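; BP_Bullet is a projectile actor that tags itself "Bullet" on BeginPlay and travels in a straight line.
; Tick moves it each frame by Direction times Speed scaled by delta time, using a swept SetActorLocation instead of a movement component.
; A Movement function holds the same logic but is not called from the event graph, and the graphs contain no hit or damage handling.
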(event `self.ReceiveBeginPlay`
  (`KismetArrayLibrary.Array_Add` (`self.Tags`) "Bullet"))

(event `self.ReceiveTick`
  (params (DeltaSeconds :type "Float (single-precision)"))
  (`self.K2_SetActorLocation` (+ (* DeltaSeconds (* (`self.Direction`) (`self.Speed`))) (`self.K2_GetActorLocation`)) true))

(fn `Movement`
  (params (DeltaSeconds :type "Float (double-precision)"))
  (`self.K2_SetActorLocation` (+ (* DeltaSeconds (* (`self.Direction`) (`self.Speed`))) (`self.K2_GetActorLocation`)) true))

(fn `UserConstructionScript`)