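; BP_Enemy is an enemy Blueprint that moves and takes damage from bullets.
; Each Tick calls Movement with the frame delta time.
; When an actor tagged Bullet begins overlapping Collision, it casts it to BP_Bullet, passes that bullet's Damage to TakeDamage and destroys the bullet.
; A failed cast only prints a debug string, and the bodies of Movement and TakeDamage are not defined here.
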(event `self.ReceiveTick`
  (params (DeltaSeconds :type "Float (single-precision)"))
  (`self.Movement` DeltaSeconds))

(event `self.Collision.OnComponentBeginOverlap`
  (params (OverlappedComponent :type "PrimitiveComponent Object Reference") (OtherActor :type "Actor Object Reference") (OtherComp :type "PrimitiveComponent Object Reference") (OtherBodyIndex :type Integer) (bFromSweep :type Boolean) (SweepResult :type "HitResult Structure (by ref)"))
  (if (`self.ActorHasTag` OtherActor "Bullet")
    (bind _asbp_bullet (cast `/Game/Blueprints/BP_Bullet` OtherActor)
      (:`then`
        (`self.TakeDamage` (`/Game/Blueprints/BP_Bullet.Damage` _asbp_bullet))
        (`self.K2_DestroyActor` OtherActor))
      (:`CastFailed`
        (`KismetSystemLibrary.PrintString` "Tag Not Found")))))

(fn `UserConstructionScript`
  (`parent.UserConstructionScript`))