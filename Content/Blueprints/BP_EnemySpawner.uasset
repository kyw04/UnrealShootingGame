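; Enemy spawner actor that periodically spawns a random enemy class from its SpawnEnemies array at its own transform.
; Tick accumulates delta time in SpawnTime until it reaches SpawnDelay, then spawns with collision handling set to always spawn.
; The timer resets to SpawnDelay minus SpawnTime, a zero or negative value, so any overshoot lengthens the next interval.
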(event `self.ReceiveTick`
  (params (DeltaSeconds :type "Float (single-precision)"))
  (bind _spawnenemies (`self.SpawnEnemies`))
  (bind _output_get (set `self.SpawnTime` (+ DeltaSeconds (`self.SpawnTime`))))
  (if (>= _output_get (`self.SpawnDelay`))
    (set `self.SpawnTime` (- (`self.SpawnDelay`) (`self.SpawnTime`)))
    (`|SpawnActorFromClass` (`|GetArrayItem` _spawnenemies (`KismetMathLibrary.RandomInteger` (`KismetArrayLibrary.Array_Length` _spawnenemies))) (`self.GetTransform`) "AlwaysSpawn" "MultiplyWithRoot" null null)))

(fn `UserConstructionScript`)