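; BP_Entity is an actor providing shared health, movement, damage, bullet spawning and death logic, with an attached health bar widget.
; BeginPlay fills health, links WBP_Hpbar to the entity and hides it until TakeDamage reveals it, reduces health and flags the hit.
; At zero health or below, OnDie sets the death flag and switches collision to the Dead profile.
; Movement sweeps along Direction, and SpawnBullet spawns a given class, owned by the entity, at BulletSpawnPosition.
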(event `self.ReceiveBeginPlay`
  (set `self.CurHealth` (`self.MaxHealth`))
  (bind _aswbp_hpbar (cast `/Game/Blueprints/WBP_Hpbar` (`WidgetComponent.GetUserWidgetObject` (`self.HP_Bar`))))
  (set `/Game/Blueprints/WBP_Hpbar.OtherActor` self _aswbp_hpbar)
  (`UserWidget.SetColorAndOpacity` :`self` _aswbp_hpbar))

(fn `Movement`
  (params (DeltaSeconds :type "Float (double-precision)"))
  (`self.K2_SetActorLocation` (+ (* DeltaSeconds (* (`self.Direction`) (`self.Speed`))) (`self.K2_GetActorLocation`)) true))

(fn `OnDie`
  (params (Attacker :type "Actor Object Reference"))
  (set `self.IsDie` true)
  (`PrimitiveComponent.SetCollisionProfileName` (`self.Collision`) "Dead" true))

(fn `SpawnBullet`
  (params (Target :type "Actor Class Reference"))
  (returns (Retrun :type "Actor Object Reference"))
  (bind _returnvalue (`|SpawnActorFromClass` Target (`SceneComponent.GetSocketTransform` (`self.Bullet Spawn Position`) "None" "RTS_World") "Undefined" "MultiplyWithRoot" self null))
  (return _returnvalue))

(fn `TakeDamage`
  (params (Value :type "Float (double-precision)") (Attacker :type "Actor Object Reference"))
  (`UserWidget.SetColorAndOpacity` (`WidgetComponent.GetUserWidgetObject` (`self.HP_Bar`)) (struct :`R` 1.0 :`G` 1.0 :`B` 1.0 :`A` 1.0))
  (bind _output_get (set `self.CurHealth` (- (`self.CurHealth`) Value)))
  (set `self.IsHit` true)
  (if (<= _output_get 0.0)
    (`self.OnDie` Attacker)))

(fn `UserConstructionScript`)