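; Player actor that moves in the Y-Z plane from axis input and spawns BP_Bullet at its transform on Fire.
; Each tick normalizes Direction, masking axes blocked by accumulated overlap normals, then passes delta time to Movement.
; Overlap begin adds hit normals; input away from a wall clears that component, as does overlap end, choosing the axis from the other actor's offset.
; Normalization is a hand-written function without a zero-length guard.
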(event `self.ReceiveTick`
  (params (DeltaSeconds :type "Float (single-precision)"))
  (if (`self.IsOverlapping`)
    ; 벽이랑 부딪히면 이동 불가
    (bind _normal (`self.Normalize` (* (- (1.0 1.0 1.0) (`KismetMathLibrary.Vector_GetAbs` (`self.OverlapHitNormal`))) (`self.Direction`))))
    (set `self.Direction` _normal)
    (else
      (bind _normal_2 (`self.Normalize` (`self.Direction`)))
      (set `self.Direction` _normal_2)))
  (`self.Movement` DeltaSeconds))

(event `InputAxis|Horizontal`
  (params (AxisValue :type "Float (single-precision)"))
  (bind (_overlaphitnormal_x _overlaphitnormal_y) (`KismetMathLibrary.BreakVector` (`self.OverlapHitNormal`)))
  (bind (_overlaphitnormal_x_2 _overlaphitnormal_y_2 _overlaphitnormal_z) (`KismetMathLibrary.BreakVector` (`self.OverlapHitNormal`)))
  (bind (_overlaphitnormal_x_3 _overlaphitnormal_y_3 _overlaphitnormal_z_2) (`KismetMathLibrary.BreakVector` (`self.OverlapHitNormal`)))
  (bind (_overlaphitnormal_x_4 _overlaphitnormal_y_4) (`KismetMathLibrary.BreakVector` (`self.OverlapHitNormal`)))
  ; 이동 방향 설정 및 부딪힌 벽이랑 반대 방향으로 움직이면 부딪힘 상쇄
  (set `self.Direction` (`KismetMathLibrary.MakeVector` 0.0 AxisValue (stale `InputAxis|Vertical` AxisValue)) :!label _label)
  (bind _result (`self.IsDirectionDifferent` AxisValue _overlaphitnormal_y_4))
  (if _result
    (set `self.OverlapHitNormal` (`KismetMathLibrary.MakeVector` _overlaphitnormal_x_3 0.0 _overlaphitnormal_z_2)))
  (bind _result_2 (`self.IsDirectionDifferent` (stale `InputAxis|Vertical` AxisValue) _overlaphitnormal_z))
  (if _result_2
    (set `self.OverlapHitNormal` (`KismetMathLibrary.MakeVector` _overlaphitnormal_x _overlaphitnormal_y))))

(event `InputAxis|Vertical`
  (params (AxisValue :type "Float (single-precision)"))
  ; 이동 방향 설정 및 부딪힌 벽이랑 반대 방향으로 움직이면 부딪힘 상쇄
  (goto _label))

(event `self.Collision.OnComponentBeginOverlap`
  (params (OverlappedComponent :type "PrimitiveComponent Object Reference") (OtherActor :type "Actor Object Reference") (OtherComp :type "PrimitiveComponent Object Reference") (OtherBodyIndex :type Integer) (bFromSweep :type Boolean) (SweepResult :type "HitResult Structure (by ref)"))
  (bind (_bblockinghit _binitialoverlap _time _distance _location _impactpoint _normal) (`GameplayStatics.BreakHitResult` SweepResult))
  ; 충돌 처리
  (if (`self.IsOverlapping`)
    (set `self.OverlapHitNormal` (+ (`self.OverlapHitNormal`) _normal))
    (else
      (set `self.OverlapHitNormal` _normal)))
  (set `self.IsOverlapping` true))

(event `self.Collision.OnComponentEndOverlap`
  (params (OverlappedComponent :type "PrimitiveComponent Object Reference") (OtherActor :type "Actor Object Reference") (OtherComp :type "PrimitiveComponent Object Reference") (OtherBodyIndex :type Integer))
  (bind (_overlaphitnormal_x _overlaphitnormal_y _overlaphitnormal_z) (`KismetMathLibrary.BreakVector` (`self.OverlapHitNormal`)))
  (bind (_returnvalue_x _returnvalue_y _returnvalue_z) (`KismetMathLibrary.BreakVector` (- (`self.K2_GetActorLocation` OtherActor) (`self.K2_GetActorLocation`))))
  ; 충돌 처리
  (if (< (`KismetMathLibrary.Abs` _returnvalue_y) (`KismetMathLibrary.Abs` _returnvalue_z))
    (set `self.OverlapHitNormal` (* (1.0 0.0 1.0) (`self.OverlapHitNormal`)))
    (else
      (set `self.OverlapHitNormal` (* (1.0 1.0 0.0) (`self.OverlapHitNormal`)))))
  (set `self.IsOverlapping` (not (and (== _overlaphitnormal_y 0.0) (== _overlaphitnormal_z 0.0)))))

(event `InputAction|Fire`
  (params (Key :type "Key Structure"))
  ; 총알 소환
  (:`Pressed`
    (`|SpawnActorFromClass` "/Game/Blueprints/BP_Bullet.BP_Bullet_C" (`self.GetTransform`) "Undefined" "MultiplyWithRoot" null null)))

(fn `IsDirectionDifferent`
  (params (A :type "Float (double-precision)") (B :type "Float (double-precision)"))
  (returns (Result :type Boolean))
  (return (< 0.0 (* A B))))

(fn `Normalize`
  (params (Default :type "Vector Structure"))
  (returns (Normal :type "Vector Structure"))
  (bind _returnvalue (`KismetMathLibrary.Sqrt` (+ (`KismetMathLibrary.MultiplyMultiply_FloatFloat` Default_X 2.0) (`KismetMathLibrary.MultiplyMultiply_FloatFloat` Default_Y 2.0) (`KismetMathLibrary.MultiplyMultiply_FloatFloat` Default_Z 2.0))))
  (return (`KismetMathLibrary.MakeVector` (/ Default_X _returnvalue) (/ Default_Y _returnvalue) (/ Default_Z _returnvalue))))

(fn `UserConstructionScript`
  (`parent.UserConstructionScript`))