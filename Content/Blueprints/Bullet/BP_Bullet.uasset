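; Bullet actor that flies along an N-point Bezier curve, then either destroys itself after one second or loops from its current location.
; BeginPlay tags it, runs the default control points through a YZ-plane rotation at zero degrees, which flattens X, and offsets them by actor location.
; Tick evaluates the Bernstein sum using a binomial helper, moves the actor with sweep at speed-scaled time, and draws debug circles.
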(event `self.ReceiveBeginPlay`
  (`KismetArrayLibrary.Array_Add` (`self.Tags`) "Bullet")
  (`self.RotateAndSetPosition` 0.0))

(event `self.ReceiveTick`
  (params (DeltaSeconds :type "Float (single-precision)"))
  ; Bezier를 이용한 총알 이동 궤적
  (for _array_element (`self.DefalutPositions`)
    (`KismetSystemLibrary.DrawDebugCircle` _array_element 10.0 12 (struct :`R` 1.0 :`G` 1.0 :`A` 1.0) 1.0 1.0))
  (bind _output_get (set `self.CurrentTime` (+ DeltaSeconds (`self.CurrentTime`))))
  (if (>= _output_get 1.0)
    (if (`self.Loop`)
      (`self.SetPosition`)
      (set `self.CurrentTime` 0.0)
      (bind _result (`self.GetBezierCurvePosition` (* (`self.CurrentTime`) (`self.Speed`)) :!label _label))
      (`self.K2_SetActorLocation` _result true)
      (`KismetSystemLibrary.DrawDebugCircle` _result 1.0 12 (struct :`R` 1.0 :`A` 1.0) 1.0 1.0)
      (else
        (`self.K2_DestroyActor`)))
    (else
      (goto _label))))

(fn `Combination`
  (params (nCi :type Integer :default 1) (n :type Integer :default 1) (i :type Integer :default 1))
  (returns (Result :type Integer))
  (for _index (range 1 (+ i 1))
    (`|VariableSetRef` nCi (* (+ (* (- i _index) -1) n) nCi))
    (`|VariableSetRef` nCi (/ nCi _index)))
  (return nCi))

(fn `GetBezierCurvePosition`
  (params (CurrentTime :type "Float (double-precision)") (Temp :type "Vector Structure"))
  (returns (Result :type "Vector Structure"))
  (bind _returnvalue (- (`KismetArrayLibrary.Array_Length` (`self.Positions`)) 1))
  (for _index (range (+ _returnvalue 1))
    (bind _result (`self.Combination` 1 _returnvalue _index))
    (bind (_returnvalue_x _returnvalue_y _returnvalue_z) (`KismetMathLibrary.BreakVector` (+ (* (* _result (`KismetMathLibrary.MultiplyMultiply_FloatFloat` (- 1.0 CurrentTime) (`KismetMathLibrary.Conv_IntToDouble` (- _returnvalue _index))) (`KismetMathLibrary.MultiplyMultiply_FloatFloat` CurrentTime (`KismetMathLibrary.Conv_IntToDouble` _index))) (`|GetArrayItem` (`self.Positions`) _index)) Temp)))
    (`KismetMathLibrary.Vector_Set` Temp _returnvalue_x _returnvalue_y _returnvalue_z))
  (return Temp))

(fn `RotateAndSetPosition`
  (params (Value :type "Float (double-precision)"))
  (bind (_returnvalue_x _returnvalue_y _returnvalue_z) (`KismetMathLibrary.BreakVector` (`self.K2_GetActorLocation`)))
  (for (_array_element _array_index) (`self.DefalutPositions`)
    (`KismetArrayLibrary.Array_Set` (`self.DefalutPositions`) _array_index (`KismetMathLibrary.MakeVector` 0.0 (- (+ (* (- (.y _array_element) _returnvalue_y) (`KismetMathLibrary.DegCos` Value)) _returnvalue_y) (* (- (.z _array_element) _returnvalue_z) (`KismetMathLibrary.DegSin` Value))) (+ (+ (* (- (.y _array_element) _returnvalue_y) (`KismetMathLibrary.DegSin` Value)) _returnvalue_z) (* (- (.z _array_element) _returnvalue_z) (`KismetMathLibrary.DegCos` Value))))))
  (`KismetArrayLibrary.Array_Set` (`self.DefalutPositions`))
  (`self.SetPosition`))

(fn `SetPosition`
  (`KismetArrayLibrary.Array_Clear` (`self.Positions`))
  (for _array_element (`self.DefalutPositions`)
    (`KismetArrayLibrary.Array_Add` (`self.Positions`) (+ _array_element (`self.K2_GetActorLocation`)))))

(fn `UserConstructionScript`)