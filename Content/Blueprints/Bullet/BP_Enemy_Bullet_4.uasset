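; BP_Enemy_Bullet_4 is an enemy bullet that bursts into a full ring of child bullets shortly after spawning.
; After a short delay on BeginPlay, it casts its owner to BP_Enemy and calls that enemy's BulletSpawn with ChildBullet in a loop.
; Each child moves to this bullet's location and is rotated to an evenly spaced angle, then the parent bullet destroys itself.
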(event `self.ReceiveBeginPlay`
  (`parent.ReceiveBeginPlay`)
  (`KismetSystemLibrary.Delay` 0.75)
  (bind _asbp_enemy (cast `/Game/Blueprints/Enemies/BP_Enemy` (`self.GetOwner`)))
  (for _index (range 15)
    (bind _retrun (`/Game/Blueprints/BP_Entity.BulletSpawn` _asbp_enemy (`self.ChildBullet`)))
    (`self.K2_SetActorLocation` _retrun (`self.K2_GetActorLocation`) false false)
    (`self.RotateAndSetPosition` _retrun (* _index 24)))
  (`self.K2_DestroyActor`))

(fn `UserConstructionScript`
  (`parent.UserConstructionScript`))