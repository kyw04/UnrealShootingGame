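; Boss enemy that stops moving shortly after spawning, takes damage from tagged bullets and shows the killing player's game over UI when it dies.
; BulletSpawnLoop picks a random bullet pattern on its first pass, then re-calls itself after delays to fire repeated rotated volleys or raised single shots.
; One pattern fires just once.
; Movement, damage handling and the trigger for the attack loop lie outside this graph.
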(event `self.ReceiveBeginPlay`
  (`parent.ReceiveBeginPlay`)
  (`KismetSystemLibrary.Delay` 2.0)
  (set `self.Speed` 0.0))

(event `self.ReceiveTick`
  (params (DeltaSeconds :type "Float (single-precision)"))
  (`parent.ReceiveTick` DeltaSeconds))

(event `self.Collision.OnComponentBeginOverlap`
  (params (OverlappedComponent :type "PrimitiveComponent Object Reference") (OtherActor :type "Actor Object Reference") (OtherComp :type "PrimitiveComponent Object Reference") (OtherBodyIndex :type Integer) (bFromSweep :type Boolean) (SweepResult :type "HitResult Structure (by ref)"))
  (if (`self.IsDie`)
    _
    (elif (`self.ActorHasTag` OtherActor "Bullet")
      (bind _asbp_bullet (cast `/Game/Blueprints/Bullet/BP_Bullet` OtherActor))
      (`self.TakeDamage` (`/Game/Blueprints/Bullet/BP_Bullet.Damage` _asbp_bullet) (`self.GetOwner` _asbp_bullet))
      (`self.K2_DestroyActor` OtherActor))))

(event `self.OnDie`
  (params (Attacker :type "Actor Object Reference"))
  (`parent.OnDie` Attacker)
  (bind _asbp_player (cast `/Game/Blueprints/BP_Player` Attacker))
  (`/Game/Blueprints/BP_Player.ShowGameOverUI` _asbp_player))

(event `self.BulletSpawnLoop`
  (bind _currentattackpattern (`self.CurrentAttackPattern`))
  (bind _bulletspawnloopindex (`self.BulletSpawnLoopIndex`))
  (bind _bulletspawnloopindex_2 (`self.BulletSpawnLoopIndex`))
  (bind _bulletspawnloopindex_3 (`self.BulletSpawnLoopIndex`))
  (bind _output (`|GetArrayItem` (`self.Bullets`) _currentattackpattern))
  (if (== (`self.BulletSpawnLoopIndex`) 1)
    (set `self.CurrentAttackPattern` (`KismetMathLibrary.RandomInteger` (`KismetArrayLibrary.Array_Length` (`self.Bullets`)))))
  (switch `int` _currentattackpattern
    (:`0`
      (for _index (range 7)
        (bind _retrun (`self.BulletSpawn` _output))
        (`self.BulletRotate` _index 10.0 _retrun))
      (if (< _bulletspawnloopindex_3 5)
        (set `self.BulletSpawnLoopIndex` (+ _bulletspawnloopindex_3 1))
        (`KismetSystemLibrary.Delay` (`self.BulletLoopDelay`))
        (`self.BulletSpawnLoop`)))
    (:`1`
      (for _index_2 (range 5)
        (bind _retrun_2 (`self.BulletSpawn` _output))
        (`self.BulletRotate` _index_2 10.0 _retrun_2))
      (if (< _bulletspawnloopindex 3)
        (set `self.BulletSpawnLoopIndex` (+ _bulletspawnloopindex 1))
        (`KismetSystemLibrary.Delay` 0.5)
        (`self.BulletSpawnLoop`)))
    (:`2`
      (bind _retrun_3 (`self.BulletSpawn` _output))
      (`self.K2_SetActorLocation` _retrun_3 (+ (0.0 0.0 150.0) (`self.K2_GetActorLocation`)) false false)
      (`/Game/Blueprints/Bullet/BP_Bullet.SetPosition` _retrun_3)
      (if (< _bulletspawnloopindex_2 10)
        (set `self.BulletSpawnLoopIndex` (+ _bulletspawnloopindex_2 1))
        (`KismetSystemLibrary.Delay` (`self.BulletLoopDelay`))
        (`self.BulletSpawnLoop`)))
    (:`3`
      (`self.BulletSpawn` _output))))

(fn `UserConstructionScript`
  (`parent.UserConstructionScript`))