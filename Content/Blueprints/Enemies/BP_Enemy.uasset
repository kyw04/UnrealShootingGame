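; Enemy actor, built on a parent class, that moves, optionally fires bullets and awards its Score to the player who kills it.
; Tick calls Movement and accumulates time to spawn bullets at a fixed delay; the SpawnBullet override sets each enemy bullet's damage.
; Tag-checked overlaps apply incoming bullet damage, or damage a touched player and kill the enemy as its own attacker, so ramming gives no score.
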(event `self.ReceiveBeginPlay`
  ; Tag 추가
  (`parent.ReceiveBeginPlay`)
  (`KismetArrayLibrary.Array_Add` (`self.Tags`) "Enemy"))

(event `self.OnDie`
  (params (Attacker :type "Actor Object Reference"))
  ; 죽였을 때 점수 추가
  (`parent.OnDie` Attacker)
  (bind _asbp_player (cast `/Game/Blueprints/BP_Player` Attacker))
  (set `/Game/Blueprints/BP_Player.Score` (+ (`/Game/Blueprints/BP_Player.Score` _asbp_player) (`self.Score`)) _asbp_player))

(event `self.Collision.OnComponentBeginOverlap`
  (params (OverlappedComponent :type "PrimitiveComponent Object Reference") (OtherActor :type "Actor Object Reference") (OtherComp :type "PrimitiveComponent Object Reference") (OtherBodyIndex :type Integer) (bFromSweep :type Boolean) (SweepResult :type "HitResult Structure (by ref)"))
  ; 충돌 처리
  (if (`self.IsDie`)
    _
    (elif (`self.ActorHasTag` OtherActor "Bullet")
      (bind _asbp_bullet (cast `/Game/Blueprints/BP_Bullet` OtherActor))
      (`self.TakeDamage` (`/Game/Blueprints/BP_Bullet.Damage` _asbp_bullet) (`self.GetOwner` _asbp_bullet))
      (`self.K2_DestroyActor` OtherActor)
      (elif (`self.ActorHasTag` OtherActor "Player")
        (bind _asbp_player (cast `/Game/Blueprints/BP_Player` OtherActor))
        (`self.TakeDamage` _asbp_player (`self.Damage`) self)
        (`self.OnDie` self)))))

(event `self.ReceiveTick`
  (params (DeltaSeconds :type "Float (single-precision)"))
  (`self.Movement` DeltaSeconds)
  ; 총알 소환
  (if (and (`self.IsSpawnBullet`) (not (`self.IsDie`)))
    (bind _output_get (set `self.BulletSpawnTime` (+ DeltaSeconds (`self.BulletSpawnTime`))))
    (if (>= _output_get (`self.BulletSpawnDelay`))
      (set `self.BulletSpawnTime` (- (`self.BulletSpawnTime`) (`self.BulletSpawnDelay`)))
      (`self.SpawnBullet` (`self.Bullet`)))))

(fn `SpawnBullet`
  (params (Target :type "Actor Class Reference"))
  (returns (Retrun :type "Actor Object Reference"))
  (bind _retrun (`parent.SpawnBullet` Target))
  (bind _asbp_enemy_bullet (cast `/Game/Blueprints/Enemies/Bullet/BP_Enemy_Bullet` _retrun))
  (set `/Game/Blueprints/Enemies/Bullet/BP_Enemy_Bullet.Damage` (`self.BulletDamage`) _asbp_enemy_bullet)
  (return _retrun))

(fn `UserConstructionScript`
  (`parent.UserConstructionScript`))