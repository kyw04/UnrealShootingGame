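; BP_EnemySpawner is an actor that periodically spawns a random enemy class from its SpawnEnemies list at its own transform.
; Tick accumulates delta time and subtracts SpawnDelay each time it is reached, so leftover time carries into the next interval.
; Spawning ignores collisions, and only enemies that cast to BP_Enemy_2 receive the Player variable as their Target.
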(event `self.ReceiveTick`
  (params (DeltaSeconds :type "Float (single-precision)"))
  (bind _spawnenemies (`self.SpawnEnemies`))
  (bind _output_get (set `self.SpawnTime` (+ DeltaSeconds (`self.SpawnTime`))))
  (if (>= _output_get (`self.SpawnDelay`))
    (set `self.SpawnTime` (- (`self.SpawnTime`) (`self.SpawnDelay`)))
    (bind _returnvalue (`|SpawnActorFromClass` (`|GetArrayItem` _spawnenemies (`KismetMathLibrary.RandomInteger` (`KismetArrayLibrary.Array_Length` _spawnenemies))) (`self.GetTransform`) "AlwaysSpawn" "MultiplyWithRoot" null null))
    (bind _asbp_enemy_2 (cast `/Game/Blueprints/Enemies/BP_Enemy_2` _returnvalue))
    (set `/Game/Blueprints/Enemies/BP_Enemy_2.Target` (`self.Player`) _asbp_enemy_2)))

(fn `UserConstructionScript`)