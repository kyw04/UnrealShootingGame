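; BP_Enemy_2 is an enemy Blueprint that keeps itself rotated relative to its player target.
; While alive, it runs the parent Tick, then casts Target to BP_Player.
; If that player is alive, it sets roll from an Atan2 of the negated direction's Y and Z, zeroing pitch and yaw, so aiming happens only in the YZ plane.
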(event `self.ReceiveTick`
  (params (DeltaSeconds :type "Float (single-precision)"))
  (bind (_returnvalue_x _returnvalue_y _returnvalue_z) (`KismetMathLibrary.BreakVector` (* (`self.Direction`) -1.0)))
  (if (not (`self.IsDie`))
    (`parent.ReceiveTick` DeltaSeconds)
    (bind _asbp_player (cast `/Game/Blueprints/BP_Player` (`self.Target`)))
    (if (not (`/Game/Blueprints/BP_Entity.IsDie` _asbp_player))
      (set `self.Direction` (`KismetMathLibrary.Normal` (- (`self.K2_GetActorLocation` (`self.Target`)) (`self.K2_GetActorLocation`))))
      (`self.K2_SetActorRotation` (`KismetMathLibrary.MakeRotator` (`KismetMathLibrary.DegAtan2` _returnvalue_y _returnvalue_z))))))

(fn `UserConstructionScript`
  (`parent.UserConstructionScript`))