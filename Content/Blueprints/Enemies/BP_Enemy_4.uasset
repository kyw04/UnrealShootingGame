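; BP_Enemy_4 is an enemy variant that fires a five-bullet spread at its target.
; Its SpawnBullet override calls the parent spawn five times and casts each result to BP_Enemy_Bullet.
; Each bullet is rotated by multiples of RotateAngle, alternating sides by loop index to form a symmetric fan around a centre shot.
; All other behavior comes from the parent class.
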(event `self.ReceiveTick`
  (params (DeltaSeconds :type "Float (single-precision)"))
  (`parent.ReceiveTick` DeltaSeconds))

(fn `SpawnBullet`
  (params (Target :type "Actor Class Reference"))
  (returns (Retrun :type "Actor Object Reference"))
  (for _index (range 5)
    (bind _retrun (`parent.SpawnBullet` Target))
    (bind _asbp_enemy_bullet (cast `/Game/Blueprints/Enemies/Bullet/BP_Enemy_Bullet` _retrun))
    (if (== (mod _index 2) 0)
      (`/Game/Blueprints/Enemies/Bullet/BP_Enemy_Bullet.RotateAndSetPosition` _asbp_enemy_bullet (* (`self.RotateAngle`) (/ _index 2)))
      (else
        (`/Game/Blueprints/Enemies/Bullet/BP_Enemy_Bullet.RotateAndSetPosition` _asbp_enemy_bullet (* (`self.RotateAngle`) (/ (+ 1 _index) 2) -1.0)))))
  (return null))

(fn `UserConstructionScript`
  (`parent.UserConstructionScript`))