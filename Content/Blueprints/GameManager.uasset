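; GameManager runs the match flow: background music, time-based scoring and the boss encounter.
; BeginPlay starts the music, and Tick adds elapsed seconds to the Player's score while the player lives, except while a valid Boss is flagged dead.
; Once the score reaches the threshold, a one-time check switches off every spawner and spawns BP_Enemy_4 as the Boss at the manager's transform.
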(event `self.ReceiveBeginPlay`
  (`GameplayStatics.PlaySound2D` "/Game/Sounds/background.background" 1.0 1.0 0.0 null null))

(event `self.ReceiveTick`
  (params (DeltaSeconds :type "Float (single-precision)"))
  (bind _player (`self.Player`))
  (bind _boss (`self.Boss`))
  (bind _returnvalue (not (`/Game/Blueprints/BP_Entity.IsDie` _player)))
  ; Boss 소환
  (if (and (not (`self.HasBoss`)) (<= 300.0 (`/Game/Blueprints/BP_Player.Score` (`self.Player`))))
    (set `self.HasBoss` true)
    (for _array_element (`self.Spawners`)
      (set `/Game/Blueprints/Enemies/BP_EnemySpawner.IsSpawning` false _array_element))
    (bind _returnvalue_2 (`|SpawnActorFromClass` "/Game/Blueprints/Enemies/BP_Enemy_4.BP_Enemy_4_C" (`self.GetTransform`) "Undefined" "MultiplyWithRoot" null null))
    (set `self.Boss` _returnvalue_2)
    (else
      ; 시간당 점수 추가
      (if (`KismetSystemLibrary.IsValid` _boss)
        (if (and (not (`/Game/Blueprints/BP_Entity.IsDie` _boss)) _returnvalue)
          (set `/Game/Blueprints/BP_Player.Score` (+ (`/Game/Blueprints/BP_Player.Score` _player) DeltaSeconds) _player :!label _label))
        (elif _returnvalue
          (goto _label))))))

(fn `UserConstructionScript`)