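; BP_Obstacles is a damageable obstacle actor that builds on inherited damage and death handling.
; Each hit runs the parent TakeDamage, then spawns the NS_Wood2 particle system, heavily scaled up, at the actor's location.
; On death it runs the parent OnDie, then destroys itself after a short delay.
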(event `/Game/Blueprints/BP_Entity.OnDie`
  (`parent.OnDie`)
  (`KismetSystemLibrary.Delay` 0.2)
  (`self.K2_DestroyActor`))

(event `/Game/Blueprints/BP_Entity.TakeDamage`
  (params (Value :type "Float (double-precision)"))
  (`parent.TakeDamage` Value)
  (`NiagaraFunctionLibrary.SpawnSystemAtLocation` "/Game/Fabs/Generic_Item_Destruction_FX/Visual_Effects/NiagaraSystem/NS_Wood2.NS_Wood2" (`self.K2_GetActorLocation`) (struct) (50.0 50.0 50.0)))

(fn `UserConstructionScript`
  (`parent.UserConstructionScript`))